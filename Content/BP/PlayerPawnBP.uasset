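; PlayerPawnBP is the player pawn Blueprint for what appears to be a snake game, exposing game state through simple getters.
; Four functions return the Hunger, Score, BonusType and SnakeDestroy values without modifying them.
; The event graph and construction script are empty, so this file contains no gameplay logic of its own.
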(event EventBeginPlay)

(event Collision|EventActorBeginOverlap
  (params (OtherActor :type Actor%20Object%20Reference)))

(event EventTick
  (params (DeltaSeconds :type Float%20%28single-precision%29)))

(fn ConstructionScript)

(fn GetHunger
  (return (Variables|Default|GetHunger)))

(fn GetScore
  (return (Variables|Default|GetScore)))

(fn GetBonusType
  (return (Variables|Default|GetBonusType)))

(fn GetSnakeDestroy
  (return (Variables|Default|GetSnakeDestroy)))